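; SmoothZoom is a Blueprint that smoothly zooms a camera by changing the arm length of a spring arm passed in through SetSpringArm.
; SmoothZoom steps the desired distance from the current, possibly mid-interpolation, arm length, clamped between min and max; a true input lengthens the arm.
; Tick eases the arm toward that distance with FInterpTo, skipping updates once within a small tolerance.
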(event `self.ReceiveTick`
  (params (DeltaSeconds :type "Float (single-precision)"))
  (if (not (`KismetMathLibrary.NearlyEqual_FloatFloat` (`SpringArmComponent.TargetArmLength` (`self.SpringArmComponent`)) (`self.DesiredDistance`) 0.5))
    (set `SpringArmComponent.TargetArmLength` (`KismetMathLibrary.FInterpTo` (`SpringArmComponent.TargetArmLength` (`self.SpringArmComponent`)) (`self.DesiredDistance`) DeltaSeconds (`self.ZoomSmoothness`)) (`self.SpringArmComponent`))))

(fn `SetSpringArm`
  (params (SpringArm :type "SpringArmComponent Object Reference"))
  (bind _output_get (set `self.SpringArmComponent` SpringArm))
  (set `self.DesiredDistance` (`SpringArmComponent.TargetArmLength` _output_get)))

(fn `SmoothZoom`
  (params (ZoomInOut :type Boolean))
  (if ZoomInOut
    (set `self.DesiredDistance` (`KismetMathLibrary.FMin` (`KismetMathLibrary.FMax` (+ (`SpringArmComponent.TargetArmLength` (`self.SpringArmComponent`)) (`self.ZoomSpeed`)) (`self.MinZoomDistance`)) (`self.MaxZoomDistance`)))
    (else
      (set `self.DesiredDistance` (`KismetMathLibrary.FMin` (`KismetMathLibrary.FMax` (- (`SpringArmComponent.TargetArmLength` (`self.SpringArmComponent`)) (`self.ZoomSpeed`)) (`self.MinZoomDistance`)) (`self.MaxZoomDistance`))))))