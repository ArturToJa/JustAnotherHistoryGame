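; RTS unit pawn with a rifle that takes AI move orders or direct player control.
; Player possession adds a camera and reticle; Space returns to the RTS pawn, and the cached previous controller re-possesses on unpossess.
; Input and UnitFire share one path through the Rifle child actor and BallisticComponent, which does not check WeaponLoaded.
; Damage goes to UnitComponent, but the alive result triggers nothing.
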(event `InputAction|Fire`
  (params (Key :type "Key Structure"))
  (bind _pitch (`self.pitch`))
  (bind (_returnvalue_x _returnvalue_y _returnvalue_z) (`KismetMathLibrary.BreakVector` (`SceneComponent.GetSocketLocation` (`self.Rifle`) "Muzzleflash")))
  ;[1 1 1] Firing
  (:`Pressed`
    (if true :!label _label
      (bind _asrifle (cast `/Game/Blueprints/Rifle` (`ChildActorComponent.ChildActor` (`self.Rifle`))))
      (set `self.isFiring` true)
      (`/Game/Blueprints/Rifle.Fire` _asrifle (`self.yaw`) _pitch)
      (`/Game/Blueprints/BallisticComponent.CalculateFire` (`self.BallisticComponent`) _pitch 450.0 (/ _returnvalue_z 100.0))
      (set `self.weaponLoaded` false)
      (`KismetSystemLibrary.Delay` 0.1)
      (set `self.isFiring` false))))

(event `Key|RightMouseButton`
  (params (Key :type "Key Structure"))
  ;[1 1 1] Aiming
  (:`Pressed`
    (set `self.isAiming` true))
  (:`Released`
    (set `self.isAiming` false)))

(event `UnitFire`
  ;[1 1 1] Firing
  (goto _label))

(event `InputAction|Reload`
  (params (Key :type "Key Structure"))
  ;[1 1 1] Reloading
  (:`Pressed`
    (set `self.isReloading` true)
    (`KismetSystemLibrary.Delay` 4.0)
    (set `self.isReloading` false)
    (set `self.weaponLoaded` true)))

(event `Key|SpaceBar`
  (params (Key :type "Key Structure"))
  ;[1 1 1] SetControlBackToRTSCamera
  (:`Pressed`
    (bind _asplayer_hud (cast `/Game/Blueprints/RTSCamera/PlayerHud` (`PlayerController.GetHUD` (`GameplayStatics.GetPlayerController` 0))))
    (`/Game/Blueprints/RTSCamera/Player.SetControlToThis` (`/Game/Blueprints/RTSCamera/PlayerHud.PlayerPawn` _asplayer_hud) null)
    (`Widget.RemoveFromParent` (`self.Widget`))
    (`ActorComponent.K2_DestroyComponent` (`self.GetComponentByClass` "/Script/Engine.CameraComponent"))))

(event `self.ReceiveBeginPlay`
  ;[1 1 1] Add rifle + reticle
  (bind _returnvalue (`|CreateWidget` "/Game/UI/Reticle.Reticle_C" (`GameplayStatics.GetPlayerController` 0)))
  (set `self.Widget` _returnvalue))

(event `self.ReceivePossessed`
  (params (NewController :type "Controller Object Reference"))
  ;[1 1 1] React to posses/unpossess
  (if (`Controller.IsPlayerController` NewController)
    (`self.CreateCamera`))
  (`self.Reset`))

(event `InputAxis|LookUp`
  (params (AxisValue :type "Float (single-precision)"))
  ;[1 1 1] Camera movement
  (bind _result (`/Engine/EditorBlueprintResources/StandardMacros.NegateFloat` (`self.GetInputAxisKeyValue`))
    (:`  `
      (`self.AddControllerPitchInput` _result))))

(event `InputAxis|LookRight`
  (params (AxisValue :type "Float (single-precision)"))
  ;[1 1 1] Camera movement
  (`self.AddControllerYawInput` (`self.GetInputAxisKeyValue`)))

(event `self.ReceiveUnpossessed`
  (params (OldController :type "Controller Object Reference"))
  ;[1 1 1] React to posses/unpossess
  (if (`Controller.IsPlayerController` OldController)
    (`Controller.Possess` (`self.ControllerRef`) self)
    (else
      (set `self.ControllerRef` OldController))))

(event `InputAxis|MoveForward`
  (params (AxisValue :type "Float (single-precision)"))
  (bind (_returnvalue_roll _returnvalue_pitch _returnvalue_yaw) (`KismetMathLibrary.BreakRotator` (`self.GetControlRotation`)))
  ;[1 1 1] Movement
  (`self.AddMovementInput` (`KismetMathLibrary.GetForwardVector` (`KismetMathLibrary.MakeRotator` 0.0 0.0 _returnvalue_yaw)) AxisValue))

(event `InputAxis|MoveRight`
  (params (AxisValue :type "Float (single-precision)"))
  (bind (_returnvalue_roll _returnvalue_pitch _returnvalue_yaw) (`KismetMathLibrary.BreakRotator` (`self.GetControlRotation`)))
  ;[1 1 1] Movement
  (`self.AddMovementInput` (`KismetMathLibrary.GetRightVector` (`KismetMathLibrary.MakeRotator` 0.0 0.0 _returnvalue_yaw)) AxisValue))

(event `self.ReceiveAnyDamage`
  (params (Damage :type "Float (single-precision)") (DamageType :type "DamageType Object Reference") (InstigatedBy :type "Controller Object Reference") (DamageCauser :type "Actor Object Reference"))
  (bind _unitcomponent (`self.UnitComponent`))
  (`/Game/Blueprints/Unit/UnitComponent.TakeDamage` _unitcomponent Damage)
  (bind _isalive (`/Game/Blueprints/Unit/UnitComponent.IsAlive` _unitcomponent))
  (if _isalive
    _))

(fn `CreateCamera`
  (bind _returnvalue (`AddComponent|NODE_AddCameraComponent-1`))
  (set `CameraComponent.bUsePawnControlRotation` true _returnvalue)
  (`SceneComponent.K2_AddLocalOffset` _returnvalue (20.0 0.0 70.0) false true)
  (bind _asrifle (cast `/Game/Blueprints/Rifle` (`ChildActorComponent.ChildActor` (`self.Rifle`))))
  (`/Game/Blueprints/Rifle.SetCamera` _asrifle _returnvalue)
  (`UserWidget.AddToViewport` (`self.Widget`) 0))

(fn `LookAtUnit`
  (params (Target :type "/Game/Blueprints/Unit/Unit Object Reference"))
  (bind (_returnvalue_roll _returnvalue_pitch _returnvalue_yaw) (`KismetMathLibrary.BreakRotator` (`KismetMathLibrary.FindLookAtRotation` (`self.K2_GetActorLocation`) (`self.K2_GetActorLocation` Target))))
  (`self.K2_SetActorRotation` (`KismetMathLibrary.RInterpTo` (`KismetMathLibrary.MakeRotator` 0.0 0.0 _returnvalue_yaw) (`self.K2_GetActorRotation`) (`GameplayStatics.GetWorldDeltaSeconds`) 3.0)))

(fn `MoveUnit`
  (params (NewPosition :type "Vector2D Structure"))
  (bind _asunit_aicontroller (cast `/Game/Blueprints/Unit/UnitAIController` (`AIBlueprintHelperLibrary.GetAIController` self)))
  (`/Game/Blueprints/Unit/UnitAIController.MoveTo` _asunit_aicontroller NewPosition))

(fn `setPitch`
  (params (pitch :type "Float (double-precision)"))
  (set `self.pitch` pitch))

(fn `setYaw`
  (params (yaw :type "Float (double-precision)"))
  (set `self.yaw` yaw))

(fn `UserConstructionScript`
  (`SceneComponent.K2_AttachToComponent` (`self.Rifle`) (`self.Mesh`) "weapon" "SnapToTarget" "SnapToTarget" "SnapToTarget" true)
  (set `self.weaponLoaded` true))