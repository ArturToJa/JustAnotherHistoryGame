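; Rifle weapon Blueprint with a prototype hitscan Fire event that prints the name of the hit actor and applies no damage.
; Fire runs a debug-drawn visibility line trace from the Muzzleflash socket along the forward vector of a camera supplied through SetCamera.
; ShowMuzzle reveals the muzzle flash through a DoOnce, but its hide and reset nodes are disconnected and Fire does not call it.
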(event `Fire`
  (bind _returnvalue (`SceneComponent.GetSocketLocation` (`self.Rifle`) "Muzzleflash"))
  (bind _outhit (`KismetSystemLibrary.LineTraceSingle` :`Start` _returnvalue :`End` (+ (* (`SceneComponent.GetForwardVector` (`self.Camera`)) 2000.0) _returnvalue) :`TraceChannel` "TraceTypeQuery1" :`DrawDebugType` "ForDuration"))
  (`KismetSystemLibrary.PrintString` (`KismetSystemLibrary.GetObjectName` (`.HitActor` (`GameplayStatics.BreakHitResult` _outhit)))))

(fn `SetCamera`
  (params (Cam :type "CameraComponent Object Reference"))
  (set `self.Camera` Cam))

(fn `ShowMuzzle`
  (`/Engine/EditorBlueprintResources/StandardMacros.DoOnce` false
    (:`Completed`
      (`SceneComponent.SetVisibility` (`self.Muzzleflash`) true false))))

(fn `UserConstructionScript`)