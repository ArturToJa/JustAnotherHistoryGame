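; Formation manages a group of player-owned Units that spawn, move and turn together as a line formation.
; SpawnFormation creates Units on row-and-column offsets from GenerateLineFormation and stores each slot in the Formation array.
; PositionFormation rotates those offsets around a target using trigonometry and saves them as temporary locations.
; MoveFormation sends Units to navigable points near those locations, aims them along the new heading, then commits the centre and rotation.
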(event `self.ReceiveTick`
  (params (DeltaSeconds :type "Float (single-precision)")))

(fn `GenerateLineFormation`
  (params (spread :type "Float (double-precision)") (unitCount :type Integer) (Width :type Integer))
  (returns (FormationPositions :type "Array of Vector Structure"))
  (locals (formationCords :type "Array of Vector Structure") (horizontalOffset :type "Float (double-precision)") (verticalOffset :type "Float (double-precision)"))
  (for _index (range unitCount)
    (if (== (mod _index Width) 0)
      (`/Engine/EditorBlueprintResources/StandardMacros.DecrementFloat` (`local.verticalOffset`)
        (:`  `
          (set `local.horizontalOffset` (+ (/ (`KismetMathLibrary.Conv_IntToDouble` Width) -2.0) 0.5))))
      (else
        (`/Engine/EditorBlueprintResources/StandardMacros.IncrementFloat` (`local.horizontalOffset`)
          (:`  `
            _))))
    (`KismetArrayLibrary.Array_Add` (`local.formationCords`) (`KismetMathLibrary.MakeVector` (* (`local.verticalOffset`) spread) (* (`local.horizontalOffset`) spread) 5.0)))
  (return (`local.formationCords`)))

(fn `MoveFormation`
  (bind _newformationrotation (`self.newFormationRotation`))
  (bind _formation (`self.formation`))
  (for (_array_element _array_index) _formation
    (bind _asunit (cast `/Game/Blueprints/Unit/Unit` (`.unit_11_4E1AD35E4CFAB93FD63E3CA9AD4C7610` (break `/Game/Blueprints/UnitFormationParam` _array_element))))
    (bind _randomlocation (`NavigationSystemV1.K2_GetRandomLocationInNavigableRadius` (`.unitTempLocation_18_3D79E72A46BE6407487E6CB5F17CE187` (break `/Game/Blueprints/UnitFormationParam` _array_element)) 5.0 null null))
    (`/Game/Blueprints/Unit/Unit.MoveUnit` _asunit (`KismetMathLibrary.MakeVector2D` (.x _randomlocation) (.y _randomlocation)))
    (`KismetArrayLibrary.Array_Set` _formation _array_index (make `/Game/Blueprints/UnitFormationParam` (break `/Game/Blueprints/UnitFormationParam` _array_element) (`.unitVector_15_890DD3EB489B28AC4768B7B81139C187` (break `/Game/Blueprints/UnitFormationParam` _array_element)) (`.unitStance_8_979CAE52438C126C31648E8FF6B00BD1` (break `/Game/Blueprints/UnitFormationParam` _array_element)) (`.unit_11_4E1AD35E4CFAB93FD63E3CA9AD4C7610` (break `/Game/Blueprints/UnitFormationParam` _array_element)) _newformationrotation (`.unitTempLocation_18_3D79E72A46BE6407487E6CB5F17CE187` (break `/Game/Blueprints/UnitFormationParam` _array_element))))
    (bind (_x_ _y_) (`self.Rotation Arrow` (.x (`.unitTempLocation_18_3D79E72A46BE6407487E6CB5F17CE187` (break `/Game/Blueprints/UnitFormationParam` _array_element))) (.y (`.unitTempLocation_18_3D79E72A46BE6407487E6CB5F17CE187` (break `/Game/Blueprints/UnitFormationParam` _array_element))) 3000.0 _newformationrotation))
    (`/Game/Blueprints/Unit/Unit.Look at Unit` _asunit (`KismetMathLibrary.MakeVector` _x_ _y_ (.z (`.unitTempLocation_18_3D79E72A46BE6407487E6CB5F17CE187` (break `/Game/Blueprints/UnitFormationParam` _array_element))))))
  (set `self.formationCenter` (`self.newFormationCenter`))
  (set `self.formationRotation` (`self.newFormationRotation`)))

(fn `Point with Rotation`
  (params (angle :type "Rotator Structure") (centerPoint :type "Vector Structure") (targetPoint :type "Vector Structure"))
  (returns (`point'` :type "Vector Structure"))
  (bind _returnvalue (`KismetMathLibrary.DegCos` angle_Yaw))
  (bind _returnvalue_2 (`KismetMathLibrary.DegSin` angle_Yaw))
  (bind _returnvalue_3 (- targetPoint_Y centerPoint_Y))
  (bind _returnvalue_4 (- targetPoint_X centerPoint_X))
  (return (`KismetMathLibrary.MakeVector` (+ (- (* _returnvalue _returnvalue_4) (* _returnvalue_2 _returnvalue_3)) centerPoint_X) (+ (* _returnvalue_4 _returnvalue_2) (* _returnvalue_3 _returnvalue) centerPoint_Y))))

(fn `PositionFormation`
  (params (target :type "Vector Structure") (rotation :type "Rotator Structure"))
  (bind _formation (`self.formation`))
  (bind _newformationcenter (`self.newFormationCenter`))
  (bind _newformationrotation (`self.newFormationRotation`))
  (set `self.newFormationRotation` rotation)
  (set `self.newFormationCenter` target)
  (for (_array_element _array_index) _formation
    (bind _point_ (`self.Point with Rotation` _newformationrotation _newformationcenter (+ (`.unitVector_15_890DD3EB489B28AC4768B7B81139C187` (break `/Game/Blueprints/UnitFormationParam` _array_element)) _newformationcenter)))
    (`KismetArrayLibrary.Array_Set` _formation _array_index (make `/Game/Blueprints/UnitFormationParam` (break `/Game/Blueprints/UnitFormationParam` _array_element) (`.unitVector_15_890DD3EB489B28AC4768B7B81139C187` (break `/Game/Blueprints/UnitFormationParam` _array_element)) (`.unitStance_8_979CAE52438C126C31648E8FF6B00BD1` (break `/Game/Blueprints/UnitFormationParam` _array_element)) (`.unit_11_4E1AD35E4CFAB93FD63E3CA9AD4C7610` (break `/Game/Blueprints/UnitFormationParam` _array_element)) _newformationrotation _point_))))

(fn `Rotation Arrow`
  (params (X :type "Float (double-precision)") (Y :type "Float (double-precision)") (range :type "Float (double-precision)") (angle :type "Rotator Structure"))
  (returns (`X'` :type "Float (double-precision)") (`Y'` :type "Float (double-precision)"))
  (return (+ X (* range (`KismetMathLibrary.DegCos` angle_Yaw))) (+ Y (* range (`KismetMathLibrary.DegSin` angle_Yaw)))))

(fn `Spawn Formation`
  (params (spread :type "Float (double-precision)") (unitCount :type Integer) (Width :type Integer) (formationStartingPoint :type "Vector Structure") (owner :type "Actor Object Reference"))
  (bind _formation (`self.formation`))
  (bind _asplayer (cast `/Game/Blueprints/RTSCamera/Player` owner))
  (bind _formationpositions (`self.GenerateLineFormation` spread unitCount Width))
  (for (_array_element _array_index) _formationpositions
    (bind _returnvalue (`|SpawnActorFromClass` "/Game/Blueprints/Unit/Unit.Unit_C" (`KismetMathLibrary.MakeTransform` (+ formationStartingPoint _array_element)) "AlwaysSpawn" "OverrideRootScale" _asplayer _asplayer null))
    (bind _returnvalue_2 (`self.K2_GetActorLocation` _returnvalue))
    (`KismetArrayLibrary.Array_Add` _formation (make `/Game/Blueprints/UnitFormationParam` _array_index _array_element "NewEnumerator0" _returnvalue (struct) _returnvalue_2))
    (set `self.formationCenter` (+ _returnvalue_2 (`self.formationCenter`))))
  (set `self.formationCenter` (/ (`self.formationCenter`) (`KismetArrayLibrary.Array_Length` _formation))))

(fn `UserConstructionScript`
  (locals (centre :type "Vector Structure"))
  (for _array_element _
    (set `local.centre` (+ (`SceneComponent.K2_GetComponentLocation` (`Character.CapsuleComponent` _array_element)) (`local.centre`)))))