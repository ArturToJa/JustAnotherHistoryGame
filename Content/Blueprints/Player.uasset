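; Player actor that acts as an edge-scrolling camera with mouse selection, in the style of a strategy game.
; Each Tick, GetDeltas compares the mouse position to a border inside the DPI-scaled viewport and returns a fixed-speed local offset, mapping screen vertical to X and horizontal to Y.
; BeginPlay enables input and shows the cursor; left mouse press and release both call SelectionMode on PlayerHud.
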(event `self.ReceiveTick`
  (params (DeltaSeconds :type "Float (single-precision)"))
  (bind _returnvalue (`WidgetLayoutLibrary.GetMousePositionOnViewport`))
  (bind _deltas (`self.GetDeltas` _returnvalue))
  (`self.K2_AddActorLocalOffset` (`KismetMathLibrary.MakeVector` (`KismetMathLibrary.BreakVector2D` _deltas) (`.Y` (`KismetMathLibrary.BreakVector2D` _deltas)))))

(event `self.ReceiveBeginPlay`
  (bind _returnvalue (`GameplayStatics.GetPlayerController` 0))
  (`self.EnableInput` _returnvalue)
  (set `PlayerController.bShowMouseCursor` true _returnvalue))

(event `Key|LeftMouseButton`
  (params (Key :type "Key Structure"))
  (:`Pressed`
    (bind _asplayer_hud (cast `/Game/Blueprints/PlayerHud` (`PlayerController.GetHUD` (`GameplayStatics.GetPlayerController` 0)) :!label _label))
    (`/Game/Blueprints/PlayerHud.SelectionMode` _asplayer_hud))
  (:`Released`
    (goto _label)))

(fn `GetDeltas`
  (params (MousePosition :type "Vector2D Structure"))
  (returns (Deltas :type "Vector2D Structure"))
  (locals (DeltaX :type "Float (double-precision)") (DeltaY :type "Float (double-precision)"))
  (set `local.DeltaX` 0.0)
  (set `local.DeltaY` 0.0)
  (bind _viewport_scaled (`self.GetViewportScaled`))
  (`|ExecutionSequence`
    (:`then_0`
      ;[1 1 1] Left-Right camera movement
      (if (< MousePosition_X (`self.BorderSize-Const`))
        (set `local.DeltaX` (+ (* (`self.CameraMoveSpeed`) -1.0) (`local.DeltaX`)))))
    (:`then_1`
      (if (> MousePosition_X (- (`KismetMathLibrary.BreakVector2D` _viewport_scaled) (`self.BorderSize-Const`)))
        (set `local.DeltaX` (+ (`self.CameraMoveSpeed`) (`local.DeltaX`)))))
    (:`then_2`
      ;[1 1 1] Up-Down camera movement
      (if (< MousePosition_Y (`self.BorderSize-Const`))
        (set `local.DeltaY` (+ (`self.CameraMoveSpeed`) (`local.DeltaY`)))))
    (:`then_3`
      (if (> MousePosition_Y (- (`.Y` (`KismetMathLibrary.BreakVector2D` _viewport_scaled)) (`self.BorderSize-Const`)))
        (set `local.DeltaY` (+ (* (`self.CameraMoveSpeed`) -1.0) (`local.DeltaY`)))))
    (:`then_4`
      (return (`KismetMathLibrary.MakeVector2D` (`local.DeltaY`) (`local.DeltaX`))))))

(fn `GetViewportScaled`
  (returns (`Viewport Scaled` :type "Vector2D Structure"))
  (bind (_returnvalue_x _returnvalue_y) (`KismetMathLibrary.BreakVector2D` (`WidgetLayoutLibrary.GetViewportSize`)))
  (bind _returnvalue (`WidgetLayoutLibrary.GetViewportScale`))
  (return (`KismetMathLibrary.MakeVector2D` (/ _returnvalue_x _returnvalue) (/ _returnvalue_y _returnvalue))))

(fn `UserConstructionScript`)