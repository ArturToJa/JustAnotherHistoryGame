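; HUD Blueprint that provides drag-box selection of Unit actors with the mouse.
; SelectionMode stores the mouse position as the anchor and toggles a gate that lets DrawHUD run the selection.
; While open, DrawHUD gathers Units between anchor and cursor, then prints each name and draws the translucent green box inside that loop.
; SetPlayerPawn stores a pawn reference.
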(event `self.ReceiveDrawHUD`
  (params (SizeX :type Integer) (SizeY :type Integer))
  (bind _anchorpoint (`self.AnchorPoint`))
  (bind (_x _y) (`KismetMathLibrary.BreakVector2D` _anchorpoint))
  (bind (_locationx _locationy) (`PlayerController.GetMousePosition` (`GameplayStatics.GetPlayerController` 0)))
  (bind (_returnvalue_x _returnvalue_y) (`KismetMathLibrary.BreakVector2D` (- (`KismetMathLibrary.MakeVector2D` _locationx _locationy) _anchorpoint)))
  (`/Engine/EditorBlueprintResources/StandardMacros.Gate` true :!label _label
    (:`Exit`
      (bind _output_get (set `self.SelectedActors` (`self.GetActorsInSelectionRectangle` "/Game/Blueprints/Unit.Unit_C" (`self.AnchorPoint`) (`KismetMathLibrary.MakeVector2D` _locationx _locationy) false)))
      (for _array_element _output_get
        (`KismetSystemLibrary.PrintString` (`KismetStringLibrary.Concat_StrStr` "Selected: " (`KismetSystemLibrary.GetDisplayName` _array_element)))
        (`self.DrawRect` (struct :`R` 0.261 :`G` 1.0 :`B` 0.235 :`A` 0.4) _x _y _returnvalue_x _returnvalue_y)))))

(event `SelectionMode`
  (bind (_locationx _locationy) (`PlayerController.GetMousePosition` (`GameplayStatics.GetPlayerController` 0)))
  (set `self.AnchorPoint` (`KismetMathLibrary.MakeVector2D` _locationx _locationy))
  (goto _label :!via `Toggle`))

(fn `SetPlayerPawn`
  (params (PlayerReference :type "/Game/Blueprints/Player Object Reference"))
  (set `self.PlayerPawn` PlayerReference))

(fn `UserConstructionScript`)